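; BP_Simple is a simple MIDI player that loads a MIDI asset on BeginPlay, starts playback and previews the score.
; Start and stop events from the Midi component switch its tick on and off, so it ticks only during performance.
; Each note event with non-zero velocity plays a short fixed-amplitude tone at the note's converted frequency.
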(event OnEvent(Midi)
  (params (track :type Integer) (note :type Integer) (velocity :type Integer) (elapsed :type Integer))
  ;[0.1203 0 1] Processed Events
  ;[1 0.8314 0.02815] Play Simple Audio
  (if (!= velocity 0)
    (Utilities|PlayAudioNote 2048.0 (Class|MidiUtils|NotetoFrequency note) 0.5)))

(event OnStop(Midi)
  (params (finished :type Boolean))
  ;[1 0 0.02122] Performance
  (Components|Tick|SetComponentTickEnabled (Variables|Default|GetMidi) false))

(event OnStart(Midi)
  (params (beginning :type Boolean))
  ;[1 0 0.02122] Performance
  (Components|Tick|SetComponentTickEnabled (Variables|Default|GetMidi) true))

(event EventBeginPlay
  (bind _midi (Variables|Default|GetMidi))
  ;[0 1 0.6045] Setup Midi
  (Components|Tick|SetComponentTickEnabled _midi false)
  (Class|MidiComponent|LoadAsset _midi (Variables|Default|GetMidi%20Asset))
  (Class|MidiComponent|Start _midi)
  ;[0.05033 1 0] Preview Midi Score
  (Class|MidiUtils|PreviewScore (Variables|/Script/MidiAsset.MidiAsset|GetData (Variables|Default|GetMidi%20Asset))))

(fn ConstructionScript)